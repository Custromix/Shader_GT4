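; BP_Cactus is an enemy cactus character that chases and attacks the player once it sees them.
; PawnSensing triggers an AI move to the player, and a successful move plays an attack montage and applies damage.
; Incoming damage drains Life, and at zero it is marked dead and stops moving.
; A separate DeathAnimation event swaps in a death material, whose height parameter Tick raises to fade it before destroying the actor.
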(event OnSeePawn(PawnSensing)
  (params (Pawn :type Pawn%20Object%20Reference))
  (if (Variables|Default|GetisAlive)
    (Variables|Default|SetisSeenPlayer true)
    (CallFunction|Follow)))

(event Custom|Follow
  (if (Variables|Default|GetisAlive)
    (AI|AIMoveTo self "0, 0, 0" (Game|GetPlayerCharacter 0) 5.0 false
      (:OnSuccess
        (Animation|PlayAnimMontage "/Game/Art/Characters/Cactus/Animations/AM_CactusAttack.AM_CactusAttack" 1.0 "None")
        (Game|Damage|ApplyDamage (Game|GetPlayerCharacter 0) 1e+01 0 0)))))

(event Custom|DeathAnimation
  (Rendering|Material|SetMaterial (Variables|Character|GetMesh) 0 "/Game/Kader/Materials/MI_CactusDeath.MI_CactusDeath")
  (Variables|Default|SetmaterialAnimationReady true))

(event EventTick
  (params (DeltaSeconds :type Float%20%28single-precision%29))
  (if (Variables|Default|GetmaterialAnimationReady)
    (bind _output_get (Variables|Default|SetHeigth (+ (Variables|Default|GetHeigth) (* DeltaSeconds (Variables|Default|GetSpeedFade)))))
    (Rendering|Material|SetScalarParameterValueonMaterials (Variables|Character|GetMesh) "Height" _output_get)
    (if (> _output_get 1.0)
      (Actor|DestroyActor))))

(event Game|Damage|EventAnyDamage
  (params (Damage :type Float%20%28single-precision%29) (DamageType :type Damage%20Type%20Object%20Reference) (InstigatedBy :type Controller%20Object%20Reference) (DamageCauser :type Actor%20Object%20Reference))
  (Variables|Default|SetLife (- (Variables|Default|GetLife) Damage))
  (if (<= (Variables|Default|GetLife) 0.0)
    (Variables|Default|SetisAlive false)
    (Components|Movement|StopMovementImmediately (Variables|Character|GetCharacterMovement))))

(fn ConstructionScript)