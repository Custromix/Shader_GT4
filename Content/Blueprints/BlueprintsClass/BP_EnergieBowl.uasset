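; BP_EnergieBowl is an energy projectile actor that flies toward a Target location and is destroyed on impact.
; The construction script applies Speed and gravity scale to its ProjectileMovement component.
; BeginPlay sets velocity along the direction to Target and rotates the actor to face it, with no homing afterward.
; A Box component hit prints a debug string, spawns the HitParticle Niagara system at the impact point and destroys the actor.
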(event OnComponentHit(Box)
  (params (HitComponent :type Primitive%20Component%20Object%20Reference) (OtherActor :type Actor%20Object%20Reference) (OtherComp :type Primitive%20Component%20Object%20Reference) (NormalImpulse :type Vector :default "0, 0, 0") (Hit :type Hit%20Result%20Structure%20%28by%20ref%29))
  (Development|PrintString "zggz")
  (Niagara|SpawnSystematLocation (Variables|ProjectileSettings|GetHitParticle) (.Location (Collision|BreakHitResult Hit)))
  (Actor|DestroyActor))

(event EventBeginPlay
  (bind _output_get (Variables|/Script/Engine.MovementComponent|SetVelocity (Variables|Default|GetProjectileMovement) (* (Math|Vector|GetUnitDirection(Vector) (Transformation|GetActorLocation) (Variables|Target|GetTarget)) (Variables|ProjectileSettings|GetSpeed))))
  (Transformation|SetActorRotation (Math|Conversions|RotationFromXVector _output_get)))

(event EventTick
  (params (DeltaSeconds :type Float%20%28single-precision%29)))

(fn ConstructionScript
  (bind _projectilemovement (Variables|Default|GetProjectileMovement))
  (Variables|/Script/Engine.ProjectileMovementComponent|SetInitialSpeed _projectilemovement (Variables|ProjectileSettings|GetSpeed))
  (Variables|/Script/Engine.ProjectileMovementComponent|SetMaxSpeed _projectilemovement (Variables|ProjectileSettings|GetSpeed))
  (Variables|/Script/Engine.ProjectileMovementComponent|SetProjectileGravityScale _projectilemovement (Variables|ProjectileSettings|GetGavity)))