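; Spawner actor from the Stylized VFX pack that repeatedly fires BP_WebShot actors for a spider web effect.
; From BeginPlay, it spawns each shot at a random nearby offset, aimed randomly within a cone around its forward vector.
; The Again event loops by calling itself after a short random delay, with no stop condition.
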(event Custom|Again
  (Game|SpawnActorfromClass "/Game/Stylized_VFX_StPack/Blueprints/UPDATE_1_3/BP_WebShot.BP_WebShot_C" (Math|Transform|MakeTransform (+ (Transformation|GetActorLocation) (* (Math|Random|RandomUnitVector) (Math|Random|RandomFloatinRange 1e+01 1e+02))) (Math|Rotator|MakeRotfromX (Math|Random|RandomUnitVectorinConeinDegrees (Transformation|GetActorForwardVector) 25.0)) "1.000000,1.000000,1.000000") "Undefined" "OverrideRootScale" 0 1.0 false 3.0 0)
  (Utilities|FlowControl|Delay (Math|Random|RandomFloatinRange 0.8 1.5))
  (CallFunction|Again))

(event EventBeginPlay
  (Game|SpawnActorfromClass "/Game/Stylized_VFX_StPack/Blueprints/UPDATE_1_3/BP_WebShot.BP_WebShot_C" (Math|Transform|MakeTransform (+ (Transformation|GetActorLocation) (* (Math|Random|RandomUnitVector) (Math|Random|RandomFloatinRange 1e+01 1e+02))) (Math|Rotator|MakeRotfromX (Math|Random|RandomUnitVectorinConeinDegrees (Transformation|GetActorForwardVector) 25.0)) "1.000000,1.000000,1.000000") "Undefined" "OverrideRootScale" 0 1.0 false 3.0 0)
  (Utilities|FlowControl|Delay (Math|Random|RandomFloatinRange 0.8 1.5))
  (CallFunction|Again))

(fn ConstructionScript)